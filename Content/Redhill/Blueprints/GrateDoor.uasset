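; GrateDoor is a sliding grate door that opens and closes through Triggeron and TriggerOff events.
; The construction script builds the grate from evenly spaced instanced static meshes, applies material overrides and places an arrow at the Offset position.
; Triggeron plays a timeline that lerps the Pivot's relative location from origin to Offset, and TriggerOff reverses it.
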(event `/ALSV4_CPP/AdvancedLocomotionV4/Blueprints/BPI/BPI_Triggerable.TriggerOn`
  (params (Instigator :type "Actor Object Reference"))
  (bind (_direction _lerp) (`Timeline|Timeline` :!label _label)
    (:`Update`
      (`SceneComponent.K2_SetRelativeLocation` (`self.Pivot`) (`KismetMathLibrary.VLerp` (0.0 0.0 0.0) (`self.Offset`) _lerp) false false))))

(event `/ALSV4_CPP/AdvancedLocomotionV4/Blueprints/BPI/BPI_Triggerable.TriggerOff`
  (params (Instigator :type "Actor Object Reference"))
  (goto _label :!via `Reverse`))

(fn `UserConstructionScript`
  (bind _instancedstaticmesh (`self.InstancedStaticMesh`))
  (`|ExecutionSequence`
    (:`then_0`
      (`InstancedStaticMeshComponent.ClearInstances` _instancedstaticmesh)
      (for _index (range (+ (`self.Count`) 1))
        (`InstancedStaticMeshComponent.AddInstance` _instancedstaticmesh (`KismetMathLibrary.MakeTransform` (* _index (`self.Spacing`)) (`self.Rotation`) (`self.Scale`)) false)))
    (:`then_1`
      (for (_array_element _array_index) (`self.MaterialsOverride`)
        (`PrimitiveComponent.SetMaterial` (`self.InstancedStaticMesh`) _array_index _array_element)))
    (:`then_2`
      (`SceneComponent.K2_SetRelativeLocationAndRotation` (`self.Arrow`) (`self.Offset`) (`KismetMathLibrary.Conv_VectorToRotator` (`KismetMathLibrary.Vector_Up`)) false false))))