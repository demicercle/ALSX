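; TeamTrigger is a team-specific trigger that declares a team win when a GrabbableActor_Chest of the matching team enters it.
; On overlap it accepts either the chest itself or an actor whose inventory holds the chest as the active weapon.
; TeamCheck compares the chest's PlayerTeam with the trigger's own and, on a match, calls ServerTeamWin on ALS_GameMode_MP.
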(event `self.ReceiveActorBeginOverlap`
  (params (OtherActor :type "Actor Object Reference"))
  (bind _asgrabbable_actor_chest (cast `/Game/Redhill/Blueprints/GrabbableActor_Chest` OtherActor)
    (:`then`
      (`self.TeamCheck` (`/Game/Redhill/Blueprints/GrabbableActor_Chest.Player Team` _asgrabbable_actor_chest)))
    (:`CastFailed`
      (bind _returnvalue (`/ALSV4_CPP/AdvancedLocomotionV4/Blueprints/Misc/ALSMacroLibrary.GetInventory` OtherActor)
        (:`Is Valid`
          (bind _weaponactor (`/ALSV4_CPP/AdvancedLocomotionV4/Blueprints/Components/InventoryComponent.Get Active Weapon` _returnvalue))
          (bind _asgrabbable_actor_chest_2 (cast `/Game/Redhill/Blueprints/GrabbableActor_Chest` _weaponactor))
          (`self.TeamCheck` (`/Game/Redhill/Blueprints/GrabbableActor_Chest.Player Team` _asgrabbable_actor_chest_2)))))))

(event `TeamCheck`
  (params (Team :type Integer))
  (if (== Team (`self.PlayerTeam`))
    (bind _asals_game_mode_mp (cast `/ALSV4_CPP/AdvancedLocomotionV4/Blueprints/GameModes/ALS_GameMode_MP` (`GameplayStatics.GetGameMode`)))
    (`/ALSV4_CPP/AdvancedLocomotionV4/Blueprints/GameModes/ALS_GameMode_MP.ServerTeamWin` _asals_game_mode_mp Team)))

(fn `UserConstructionScript`)