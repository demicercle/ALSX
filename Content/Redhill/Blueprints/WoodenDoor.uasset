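; WoodenDoor is a two-panel sliding door Blueprint that opens and closes in response to trigger events.
; Triggeron and TriggerOff set and clear the IsOpen flag.
; Tick snaps both panels between closed and open relative positions along Y every frame, with no interpolation or sweep.
; The construction script assigns the Mesh variable to the first panel only.
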(event `self.ReceiveTick`
  (params (DeltaSeconds :type "Float (single-precision)"))
  (`parent.ReceiveTick` DeltaSeconds)
  (`SceneComponent.K2_SetRelativeLocation` (`self.StaticMesh`) (`KismetMathLibrary.SelectVector` (0.0 -200.0 -100.0) (0.0 -100.0 -100.0) (`self.IsOpen`)) false false)
  (`SceneComponent.K2_SetRelativeLocation` (`self.StaticMesh1`) (`KismetMathLibrary.SelectVector` (0.0 200.0 -100.0) (0.0 100.0 -100.0) (`self.IsOpen`)) false false))

(event `/ALSV4_CPP/AdvancedLocomotionV4/Blueprints/BPI/BPI_Triggerable.TriggerOff`
  (params (Instigator :type "Actor Object Reference"))
  (set `self.IsOpen` false))

(event `/ALSV4_CPP/AdvancedLocomotionV4/Blueprints/BPI/BPI_Triggerable.TriggerOn`
  (params (Instigator :type "Actor Object Reference"))
  (set `self.IsOpen` true))

(fn `UserConstructionScript`
  (`parent.UserConstructionScript`)
  (`StaticMeshComponent.SetStaticMesh` (`self.StaticMesh`) (`self.Mesh`)))