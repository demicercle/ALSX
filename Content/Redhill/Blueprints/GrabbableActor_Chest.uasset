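; Grabbable chest actor that takes on the team of the player it is parented to.
; Each tick, after the parent tick, it looks for a PlayerComponent on ParentActor, sets the mesh to the blue or red material by PlayerTeam, and copies that team.
; A reset to the neutral material and no team exists but is unwired, so this graph never clears the team.
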(event `self.ReceiveTick`
  (params (DeltaSeconds :type "Float (single-precision)"))
  (bind _parentactor (`self.ParentActor`))
  (bind _returnvalue (`self.GetComponentByClass` _parentactor "/ALSV4_CPP/AdvancedLocomotionV4/Blueprints/Components/PlayerComponent.PlayerComponent_C"))
  (bind _playerteam (`/ALSV4_CPP/AdvancedLocomotionV4/Blueprints/Components/PlayerComponent.PlayerTeam` _returnvalue))
  (`parent.ReceiveTick` DeltaSeconds)
  (`/Engine/EditorBlueprintResources/StandardMacros.IsValid` _parentactor
    (:`Is Valid`
      (`/Engine/EditorBlueprintResources/StandardMacros.IsValid` _returnvalue
        (:`Is Valid`
          (`PrimitiveComponent.SetMaterial` (`self.StaticMesh`) 0 (select `int` _playerteam :`0` "/Game/Redhill/Meshes/Fantasy_Brown_08_BLU.Fantasy_Brown_08_BLU" :`1` "/Game/Redhill/Meshes/Fantasy_Brown_08_RED.Fantasy_Brown_08_RED" :!type "MaterialInterface Object Reference"))
          (set `self.Player Team` _playerteam))))))

(fn `UserConstructionScript`
  (`parent.UserConstructionScript`))