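; LootCrate is an interactable crate that supplies the interacting actor with archery gear.
; On the interactable component's interact event, it looks up the instigator's inventory component and does nothing if none exists.
; It gives a bow only if none is found, then tops arrows up to a cap of five, sheathed, through the inventory's server give-equipment calls.
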(event `self.InteractableComponent.OnInteracted`
  (params (Instigator :type "Actor Object Reference"))
  (bind _returnvalue (`self.GetComponentByClass` Instigator "/ALSV4_CPP/AdvancedLocomotionV4/Blueprints/Components/InventoryComponent.InventoryComponent_C"))
  (`/Engine/EditorBlueprintResources/StandardMacros.IsValid` _returnvalue
    (:`Is Valid`
      (`|ExecutionSequence`
        (:`then_0`
          (bind (_equippableactors _success) (`/ALSV4_CPP/AdvancedLocomotionV4/Blueprints/Components/InventoryComponent.GetEquipment` _returnvalue "/ALSV4_CPP/AdvancedLocomotionV4/Blueprints/Actors/EquippableActor_Bow.EquippableActor_Bow_C" "None"))
          (if (not _success)
            (`/ALSV4_CPP/AdvancedLocomotionV4/Blueprints/Components/InventoryComponent.ServerGiveEquipment` _returnvalue "/ALSV4_CPP/AdvancedLocomotionV4/Blueprints/Actors/EquippableActor_Bow.EquippableActor_Bow_C" 1 1 false)))
        (:`then_1`
          (bind (_equippableactors_2 _success_2 _count) (`/ALSV4_CPP/AdvancedLocomotionV4/Blueprints/Components/InventoryComponent.GetEquipment` _returnvalue "/ALSV4_CPP/AdvancedLocomotionV4/Blueprints/Actors/ItemActor_Arrow.ItemActor_Arrow_C" "None"))
          (bind _returnvalue_2 (- 5 _count))
          (if (> _returnvalue_2 0)
            (`/ALSV4_CPP/AdvancedLocomotionV4/Blueprints/Components/InventoryComponent.ServerGiveEquipment` _returnvalue "/ALSV4_CPP/AdvancedLocomotionV4/Blueprints/Actors/ItemActor_Arrow.ItemActor_Arrow_C" _returnvalue_2 5 true)))))))

(fn `UserConstructionScript`)