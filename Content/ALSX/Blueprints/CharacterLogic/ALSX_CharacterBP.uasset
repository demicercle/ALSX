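; ALSX player character that adds inventory items and interaction to its parent locomotion character, with input to cycle, use, drop and interact.
; Tick polls the inventory's active item, and change-guarded setters pair Equip/Unequip and StartUse/StopUse calls.
; Item data drives the overlay state and the mesh, animation and hand of the held object.
; Inventory changes also send the overlay to the server and add or destroy the MantleComponent as the item allows.
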(event `InputAction|NextItem`
  (params (Key :type "Key Structure"))
  (:`Pressed`
    (`/Game/ALSX/Blueprints/Inventory/ALSX_InventoryComponent.CycleItem` (`self.Inventory`) 1)))

(event `InputAction|PrevItem`
  (params (Key :type "Key Structure"))
  (:`Pressed`
    (`/Game/ALSX/Blueprints/Inventory/ALSX_InventoryComponent.CycleItem` (`self.Inventory`) -1)))

(event `self.ReceiveTick`
  (params (DeltaSeconds :type "Float (single-precision)"))
  (`parent.ReceiveTick` DeltaSeconds)
  (`self.UpdateEquippedItem`))

(event `InputAction|UseItem`
  (params (Key :type "Key Structure"))
  (:`Pressed`
    (`self.UpdateUsedItem` true))
  (:`Released`
    (`self.UpdateUsedItem` false)))

(event `InputAction|DropItem`
  (params (Key :type "Key Structure"))
  (bind _equippeditem (`self.EquippedItem`))
  (:`Pressed`
    (`/Engine/EditorBlueprintResources/StandardMacros.IsValid` _equippeditem
      (:`Is Valid`
        (`/Game/ALSX/Blueprints/Inventory/ALSX_InventoryItem.Drop` _equippeditem (`KismetMathLibrary.MakeTransform` (`KismetMathLibrary.TransformLocation` (`self.GetTransform`) (`KismetMathLibrary.MakeVector` (`self.DropDistance`)))) 0.0)))))

(event `InputAction|Interact`
  (params (Key :type "Key Structure"))
  (bind _interactioncomponent_0 (`self.InteractionComponent_0`))
  (:`Pressed`
    (`/Game/ALSX/Blueprints/ALSX_InteractionComponent.Interact` _interactioncomponent_0 true))
  (:`Released`
    (`/Game/ALSX/Blueprints/ALSX_InteractionComponent.Interact` _interactioncomponent_0 false)))

(fn `OnInventoryChanged`
  (bind _returnvalue (`self.GetComponentByClass` "/ALSV4_CPP/AdvancedLocomotionV4/Blueprints/Components/MantleComponent.MantleComponent_C"))
  (bind _output (`/Game/ALSX/Blueprints/Inventory/ALSX_InventoryComponent.GetActiveItem` (`self.Inventory`)))
  (`/Engine/EditorBlueprintResources/StandardMacros.IsValid` _output
    (:`Is Valid`
      (bind _itemdata (`/Game/ALSX/Blueprints/Inventory/ALSX_InventoryItem.ItemData` _output))
      (bind _overlaystate (`/Game/ALSX/Blueprints/Inventory/ALSX_ItemData.OverlayState` _itemdata))
      (`self.Server_SetOverlayState` _overlaystate)
      (`self.SetOverlayState` _overlaystate)
      (if (`/Game/ALSX/Blueprints/Inventory/ALSX_ItemData.CanMantleOrClimb` _itemdata)
        (`/Engine/EditorBlueprintResources/StandardMacros.IsValid` _returnvalue :!label _label
          (:`Is Not Valid`
            (`AddComponent|NODE_AddMantleComponent-0`)))
        (else
          (`/Engine/EditorBlueprintResources/StandardMacros.IsValid` _returnvalue
            (:`Is Valid`
              (`ActorComponent.K2_DestroyComponent` _returnvalue))))))
    (:`Is Not Valid`
      (`self.Server_SetOverlayState` "Default")
      (`self.SetOverlayState` "Default")
      (goto _label))))

(fn `OnUpdateHeldObject`
  (bind _equippeditem (`self.EquippedItem`))
  (bind _itemdata (`/Game/ALSX/Blueprints/Inventory/ALSX_InventoryItem.ItemData` _equippeditem))
  (`/Engine/EditorBlueprintResources/StandardMacros.IsValid` _equippeditem
    (:`Is Valid`
      (`self.AttachToHand` (`/Game/ALSX/Blueprints/Inventory/ALSX_ItemData.StaticMesh` _itemdata) (`/Game/ALSX/Blueprints/Inventory/ALSX_ItemData.SkeletalMesh` _itemdata) (`/Game/ALSX/Blueprints/Inventory/ALSX_ItemData.AnimClass` _itemdata) (`/Game/ALSX/Blueprints/Inventory/ALSX_ItemData.LeftHand` _itemdata) (`/Game/ALSX/Blueprints/Inventory/ALSX_ItemData.HandOffset` _itemdata)))
    (:`Is Not Valid`
      (`parent.OnUpdateHeldObject`))))

(fn `SetEquippedItem`
  (params (NewItem :type "/Game/ALSX/Blueprints/Inventory/ALSX_InventoryItem Object Reference"))
  (bind _equippeditem (`self.EquippedItem`))
  (bind _equippeditem_2 (`self.EquippedItem`))
  (if (not (== NewItem (`self.EquippedItem`)))
    (`|ExecutionSequence`
      (:`then_0`
        (`/Engine/EditorBlueprintResources/StandardMacros.IsValid` _equippeditem
          (:`Is Valid`
            (`/Game/ALSX/Blueprints/Inventory/ALSX_InventoryItem.Unequip` _equippeditem)
            (`self.SetUsedItem` null))))
      (:`then_1`
        (set `self.EquippedItem` NewItem))
      (:`then_2`
        (`/Engine/EditorBlueprintResources/StandardMacros.IsValid` _equippeditem_2
          (:`Is Valid`
            (`self.SetOverlayState` (`/Game/ALSX/Blueprints/Inventory/ALSX_ItemData.OverlayState` (`/Game/ALSX/Blueprints/Inventory/ALSX_InventoryItem.ItemData` _equippeditem_2)))
            (`/Game/ALSX/Blueprints/Inventory/ALSX_InventoryItem.Equip` _equippeditem_2))
          (:`Is Not Valid`
            (`self.SetOverlayState` "Default")))))))

(fn `SetUsedItem`
  (params (NewItem :type "/Game/ALSX/Blueprints/Inventory/ALSX_InventoryItem Object Reference"))
  (bind _useditem (`self.UsedItem`))
  (bind _useditem_2 (`self.UsedItem`))
  (if (not (== NewItem (`self.UsedItem`)))
    (`|ExecutionSequence`
      (:`then_0`
        (`/Engine/EditorBlueprintResources/StandardMacros.IsValid` _useditem
          (:`Is Valid`
            (`/Game/ALSX/Blueprints/Inventory/ALSX_InventoryItem.StopUse` _useditem))))
      (:`then_1`
        (set `self.UsedItem` NewItem))
      (:`then_2`
        (`/Engine/EditorBlueprintResources/StandardMacros.IsValid` _useditem_2
          (:`Is Valid`
            (`/Game/ALSX/Blueprints/Inventory/ALSX_InventoryItem.StartUse` _useditem_2)))))))

(fn `UpdateEquippedItem`
  (bind _output (`/Game/ALSX/Blueprints/Inventory/ALSX_InventoryComponent.GetActiveItem` (`self.Inventory`)))
  (`self.SetEquippedItem` _output))

(fn `UpdateUsedItem`
  (params (InputPressed :type Boolean))
  (if InputPressed
    (`self.SetUsedItem` (`self.EquippedItem`))
    (else
      (`self.SetUsedItem` null))))

(fn `UserConstructionScript`
  (`parent.UserConstructionScript`))