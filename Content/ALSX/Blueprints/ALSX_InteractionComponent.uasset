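; ALSX interaction component that finds the nearest interactable actor around its owner and lets the owner start or stop interacting with it.
; Each Tick runs a sphere overlap at an owner-relative offset and keeps the horizontally closest actor that implements BPI_Interactable and accepts interaction.
; The chosen target is outlined with a debug box, and the search sphere is optionally drawn.
; Interact forwards start or stop interface messages to that target.
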(event `self.ReceiveTick`
  (params (DeltaSeconds :type "Float (single-precision)"))
  (bind _returnvalue (`self.GetOwner`))
  (bind _returnvalue_2 (`self.GetOwner`))
  (bind _interactable (`self.Interactable`))
  (bind _sphere_radius (`self.Sphere Radius`))
  (bind _interactable_2 (`self.Interactable`))
  (bind (_origin _boxextent) (`Actor.GetActorBounds` _interactable_2 false false))
  (bind _returnvalue_3 (`KismetMathLibrary.TransformLocation` (`Actor.GetTransform` _returnvalue_2) (`self.Offset`)))
  (`|ExecutionSequence`
    (:`then_0`
      (if (`self.DrawDebugSphere`)
        (`KismetSystemLibrary.DrawDebugSphere` _returnvalue_3 _sphere_radius 12 (struct :`R` 1.0 :`G` 1.0 :`B` 1.0 :`A` 1.0) 0.0 1.0)))
    (:`then_1`
      (set `self.Interactable` null)
      (bind _outactors (`KismetSystemLibrary.SphereOverlapActors` _returnvalue_3 _sphere_radius (`|MakeArray` "ObjectTypeQuery2" "ObjectTypeQuery3" :!type "EObjectTypeQuery Enum") "/Script/Engine.Actor" (`|MakeArray` _returnvalue_2)))
      (for _array_element _outactors
        (`/Engine/EditorBlueprintResources/StandardMacros.IsValid` _interactable
          (:`Is Valid`
            (if (> (`Actor.GetHorizontalDistanceTo` _interactable _returnvalue) (`Actor.GetHorizontalDistanceTo` _array_element _returnvalue))
              (if (`KismetSystemLibrary.DoesImplementInterface` _array_element "/Game/ALSX/Blueprints/BPI_Interactable.BPI_Interactable_C") :!label _label
                (bind _success (message `/Game/ALSX/Blueprints/BPI_Interactable.CanBeInteracted` _array_element (`self.GetOwner`)))
                (if _success
                  (set `self.Interactable` _array_element)))))
          (:`Is Not Valid`
            (goto _label))))
      (`/Engine/EditorBlueprintResources/StandardMacros.IsValid` _interactable_2
        (:`Is Valid`
          (`KismetSystemLibrary.DrawDebugBox` _origin _boxextent (struct :`G` 0.45051 :`B` 1.0 :`A` 1.0) (struct) 0.0 1.0))))))

(fn `Interact`
  (params (Value :type Boolean))
  (bind _returnvalue (`self.GetOwner`))
  (bind _interactable (`self.Interactable`))
  (`/Engine/EditorBlueprintResources/StandardMacros.IsValid` _interactable
    (:`Is Valid`
      (if Value
        (message `/Game/ALSX/Blueprints/BPI_Interactable.StartInteract` _interactable _returnvalue)
        (else
          (message `/Game/ALSX/Blueprints/BPI_Interactable.StopInteract` _interactable _returnvalue))))))