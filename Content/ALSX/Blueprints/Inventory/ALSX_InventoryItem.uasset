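; Base inventory item actor for the ALSX inventory, holding its ItemData and tracking equipped and in-use state.
; Init assigns the data, while Equip, Unequip, StartUse and StopUse only toggle the state flags.
; Drop, if the data allows it, spawns the data's pickup class with a copy of ItemData, optionally traces down to snap it onto world-static ground, then destroys the item.
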(fn `Drop`
  (params (SpawnTransform :type "Transform Structure") (GroundDistance :type "Float (double-precision)"))
  (returns (Success :type Boolean))
  (bind _returnvalue (`self.GetOwner`))
  (bind _location (.location SpawnTransform))
  (bind _itemdata (`self.ItemData`))
  (if (`/Game/ALSX/Blueprints/Inventory/ALSX_ItemData.CanBeDropped` _itemdata)
    (bind _returnvalue_2 (`|SpawnActorFromClass` (`/Game/ALSX/Blueprints/Inventory/ALSX_ItemData.PickupClass` _itemdata) SpawnTransform "AlwaysSpawn" "OverrideRootScale" _returnvalue (cast `Pawn` _returnvalue :!pure true)))
    (set `/Game/ALSX/Blueprints/Inventory/ALSX_PickupItem.ItemData` (`self.ItemData`) _returnvalue_2)
    (`|ExecutionSequence`
      (:`then_0`
        (if (> GroundDistance 0.0)
          (bind (_outhit _returnvalue_3) (`KismetSystemLibrary.LineTraceSingleForObjects` :`Start` _location :`End` (- _location (`KismetMathLibrary.MakeVector` 0.0 0.0 GroundDistance)) :`ObjectTypes` (`|MakeArray` "ObjectTypeQuery1" :!type "EObjectTypeQuery Enum") :`DrawDebugType` "ForDuration"))
          (if _returnvalue_3
            (`self.K2_SetActorLocation` _returnvalue_2 (`.Location` (`GameplayStatics.BreakHitResult` _outhit)) true false))))
      (:`then_1`
        (`self.K2_DestroyActor`)
        (return true)))
    (else
      (return false))))

(fn `Equip`
  (set `self.IsEquipped` true))

(fn `Init`
  (params (ItemData :type "/Game/ALSX/Blueprints/Inventory/ALSX_ItemData Object Reference"))
  (set `self.ItemData` ItemData))

(fn `StartUse`
  (set `self.IsUsed` true))

(fn `StopUse`
  (set `self.IsUsed` false))

(fn `Unequip`
  (set `self.IsEquipped` false))

(fn `UserConstructionScript`)