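; World pickup actor for an item data asset, which it adds to the ALSX inventory component of the actor picking it up, then destroys itself.
; UpdateMesh shows the item's static or skeletal mesh, optionally auto-scaled and centered to fit the Sphere component.
; Pickup triggers on overlap, gated until shortly after BeginPlay, or through interaction when RequireInput is set.
; Tick moves it downward with a swept offset, and it destroys itself at start without valid ItemData.
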(event `self.ReceiveBeginPlay`
  (`KismetSystemLibrary.Delay` 0.2)
  (`/Engine/EditorBlueprintResources/StandardMacros.IsValid` (`self.ItemData`)
    (:`Is Valid`
      (`self.UpdateMesh`)
      (goto _label :!via `Open`))
    (:`Is Not Valid`
      (`self.K2_DestroyActor`))))

(event `self.ReceiveActorBeginOverlap`
  (params (OtherActor :type "Actor Object Reference"))
  (`/Engine/EditorBlueprintResources/StandardMacros.Gate` true :!label _label
    (:`Exit`
      (if (`self.Overlap`)
        (`self.TryPickup` OtherActor)))))

(event `/Game/ALSX/Blueprints/BPI_Interactable.StartInteract`
  (params (Instigator :type "Actor Object Reference"))
  (if (`self.RequireInput`)
    (`self.TryPickup` Instigator)))

(event `self.ReceiveTick`
  (params (DeltaSeconds :type "Float (single-precision)"))
  (`self.K2_AddActorWorldOffset` (`KismetMathLibrary.MakeVector` 0.0 0.0 (* DeltaSeconds (`self.FallVelocity`) -1.0)) true))

(fn `CanBeInteracted`
  (params (Instigator :type "Actor Object Reference"))
  (returns (Success :type Boolean))
  (return (`self.RequireInput`)))

(fn `ResizeComponent`
  (params (InBoxSphereBounds :type "BoxSphereBounds Structure (by ref)") (Component :type "SceneComponent Object Reference"))
  (bind (_origin _boxextent _sphereradius) (`KismetMathLibrary.BreakBoxSphereBounds` InBoxSphereBounds))
  (bind _sphere (`self.Sphere`))
  (bind _staticmesh (`self.StaticMesh`))
  (bind (_origin_2 _boxextent_2 _sphereradius_2) (`KismetSystemLibrary.GetComponentBounds` _sphere))
  (`SceneComponent.SetRelativeScale3D` _staticmesh (`KismetMathLibrary.SelectVector` (`KismetMathLibrary.Conv_DoubleToVector` (/ _sphereradius_2 _sphereradius)) (1.0 1.0 1.0) (`self.AutoSize`)))
  (`SceneComponent.SetRelativeScale3D` Component (`KismetMathLibrary.SelectVector` (`KismetMathLibrary.Conv_DoubleToVector` (/ _sphereradius_2 _sphereradius)) (1.0 1.0 1.0) (`self.AutoSize`)))
  (`SceneComponent.K2_SetRelativeLocationAndRotation` :`self` _staticmesh :`NewLocation` (`KismetMathLibrary.SelectVector` (- (`KismetMathLibrary.InverseTransformLocation` (`SceneComponent.K2_GetComponentToWorld` _sphere) _origin_2) _origin) (0.0 0.0 0.0) (`self.AutoCenter`)))
  (`SceneComponent.K2_SetRelativeLocationAndRotation` :`self` Component :`NewLocation` (`KismetMathLibrary.SelectVector` (- (`KismetMathLibrary.InverseTransformLocation` (`SceneComponent.K2_GetComponentToWorld` _sphere) _origin_2) _origin) (0.0 0.0 0.0) (`self.AutoCenter`))))

(fn `TryPickup`
  (params (Actor :type "Actor Object Reference"))
  (returns (Success :type Boolean))
  (bind _returnvalue (`self.GetComponentByClass` Actor "/Game/ALSX/Blueprints/Inventory/ALSX_InventoryComponent.ALSX_InventoryComponent_C"))
  (`/Engine/EditorBlueprintResources/StandardMacros.IsValid` _returnvalue
    (:`Is Valid`
      (bind _success (`/Game/ALSX/Blueprints/Inventory/ALSX_InventoryComponent.AddItem` _returnvalue (`self.ItemData`)))
      (if _success
        (`self.K2_DestroyActor`)
        (return true)
        (else
          _)))
    (:`Is Not Valid`
      _))
  (return false))

(fn `UpdateMesh`
  (bind _itemdata (`self.ItemData`))
  (bind _staticmesh (`self.StaticMesh`))
  (bind _skeletalmesh (`self.SkeletalMesh`))
  (bind _skeletalmesh_2 (`/Game/ALSX/Blueprints/Inventory/ALSX_ItemData.SkeletalMesh` _itemdata))
  (bind _pickupmesh (`/Game/ALSX/Blueprints/Inventory/ALSX_ItemData.PickupMesh` _itemdata))
  (`/Engine/EditorBlueprintResources/StandardMacros.IsValid` _itemdata
    (:`Is Valid`
      (`SceneComponent.SetVisibility` _staticmesh true false)
      (`SceneComponent.SetVisibility` (`self.SkeletalMesh`) true false)
      (`|ExecutionSequence`
        (:`then_0`
          (`SkinnedMeshComponent.SetSkinnedAssetAndUpdate` _skeletalmesh _skeletalmesh_2 true)
          (`/Engine/EditorBlueprintResources/StandardMacros.IsValid` _skeletalmesh_2
            (:`Is Valid`
              (`self.ResizeComponent` (`SkeletalMesh.GetBounds` _skeletalmesh_2) _skeletalmesh))))
        (:`then_1`
          (bind _returnvalue (`StaticMeshComponent.SetStaticMesh` _staticmesh _pickupmesh))
          (if (and _returnvalue (`KismetSystemLibrary.IsValid` _pickupmesh))
            (`self.ResizeComponent` (`StaticMesh.GetBounds` _pickupmesh) (`self.StaticMesh`))))))
    (:`Is Not Valid`
      (`SceneComponent.SetVisibility` (`self.StaticMesh`) false false)
      (`SceneComponent.SetVisibility` (`self.SkeletalMesh`) false false))))

(fn `UserConstructionScript`
  (`self.UpdateMesh`))